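; A projectile actor that triggers area damage and destroys itself when it hits something.
; Its mesh ignores the owner while moving, and on hit a debug-drawn sphere overlap searches for pawn components around it, excluding the owner.
; Each overlap runs a Weight-based damage call credited to the first player controller, though no damaged actor is set, then destroys the projectile, as does finding no overlaps.
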(event Collision|EventHit
  (params (MyComp :type Primitive%20Component%20Object%20Reference) (Other :type Actor%20Object%20Reference) (OtherComp :type Primitive%20Component%20Object%20Reference) (bSelfMoved :type Boolean) (HitLocation :type Vector :default "0, 0, 0") (HitNormal :type Vector :default "0, 0, 0") (NormalImpulse :type Vector :default "0, 0, 0") (Hit :type Hit%20Result%20Structure%20%28by%20ref%29))
  (bind _returnvalue (Transformation|GetActorLocation))
  (bind (_outcomponents _returnvalue_2) (Collision|SphereOverlapComponents _returnvalue 1.5e+02 (Utilities|Array|MakeArray "ObjectTypeQuery3") 0 (Utilities|Array|MakeArray (Components|GetOwner))))
  (Rendering|Debug|DrawDebugSphere _returnvalue 1.5e+02 12 "(R=1.000000,G=0.000000,B=0.132013,A=1.000000)" 2.0 1.0)
  (if _returnvalue_2
    (for _array_element _outcomponents
      (Game|Damage|ApplyDamage 0 (Math|Conversions|ToFloat(Integer) (Variables|Default|GetWeight)) (Game|GetPlayerController 0) (Components|GetOwner))
      (Actor|DestroyActor))
    (else
      (Actor|DestroyActor))))

(event EventBeginPlay
  (Collision|IgnoreActorwhenMoving (Variables|Default|GetStaticMesh) (Components|GetOwner) true))

(fn ConstructionScript)