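; Master interaction actor, a base for objects the main character activates by entering a collision volume.
; On overlap it stores the character reference and branches on InteractType: Interaction enables player input on the actor, while Trigger calls TriggerInteraction immediately.
; Leaving the volume clears the reference and either disables input or calls TriggerdeInteraction.
; No input handling is implemented in this Blueprint itself.
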(event OnComponentBeginOverlap(Collision)
  (params (OverlappedComponent :type Primitive%20Component%20Object%20Reference) (OtherActor :type Actor%20Object%20Reference) (OtherComp :type Primitive%20Component%20Object%20Reference) (OtherBodyIndex :type Integer) (bFromSweep :type Boolean) (SweepResult :type Hit%20Result%20Structure%20%28by%20ref%29))
  (bind _asmain_character (Utilities|Casting|CastToMain_character OtherActor))
  (Variables|Default|SetAs%20Main%20Character _asmain_character)
  (switch Utilities|FlowControl|Switch|SwitchonActor_Type (Variables|Default|GetInteract_Type)
    (:NewEnumerator0
      (Input|EnableInput (Game|GetPlayerController 0)))
    (:NewEnumerator1
      (Default|CallTriggerInteraction))))

(event OnComponentEndOverlap(Collision)
  (params (OverlappedComponent :type Primitive%20Component%20Object%20Reference) (OtherActor :type Actor%20Object%20Reference) (OtherComp :type Primitive%20Component%20Object%20Reference) (OtherBodyIndex :type Integer))
  (Utilities|Casting|CastToMain_character OtherActor)
  (Variables|Default|SetAs%20Main%20Character 0)
  (switch Utilities|FlowControl|Switch|SwitchonActor_Type (Variables|Default|GetInteract_Type)
    (:NewEnumerator0
      (Input|DisableInput (Game|GetPlayerController 0)))
    (:NewEnumerator1
      (Default|CallTriggerdeInteraction))))

(fn ConstructionScript)