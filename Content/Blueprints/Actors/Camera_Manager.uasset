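; Side-scrolling camera actor that makes itself the player's view target and follows ActorFollow along X and Z at a fixed Y offset.
; Each tick it moves only when the target leaves the X or Z dead zone.
; A FixedZValue other than the sentinel 415 locks the height instead.
; The construction script pre-positions the camera, pitched slightly down and yawed toward the target.
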(event EventBeginPlay
  (Game|Player|SetViewTargetwithBlend (Game|GetPlayerController 0) self 0.0 "VTBlend_Linear" 0.0 false))

(event EventTick
  (params (DeltaSeconds :type Float%20%28single-precision%29))
  (bind _newx (CallFunction|GetNewXValue))
  (Variables|Default|SetCameraX _newx)
  (bind _newx_2 (CallFunction|GetNewZValue))
  (Variables|Default|SetCameraZ _newx_2)
  (Transformation|SetActorLocation (Math|Vector|MakeVector (Variables|Default|GetCameraX) (Variables|Default|GetYOffset) (Variables|Default|GetCameraZ)) false false))

(fn ConstructionScript
  (bind _actorfollow (Variables|Default|GetActorFollow))
  (bind _returnvalue (Transformation|GetActorLocation _actorfollow))
  (bind (_x _y _z) (Math|Vector|BreakVector _returnvalue))
  (Utilities|IsValid _actorfollow
    (:Is%20Valid
      (bind _output_get (Variables|Default|SetCameraX _x))
      (if (!= (Variables|Default|GetFixedZValue) 415.0)
        (Variables|Default|SetCameraZ (Variables|Default|GetFixedZValue))
        (else
          (bind _output_get_2 (Variables|Default|SetCameraZ (+ _z (Variables|Default|GetZDead_Zone))))))
      (Transformation|SetActorLocation (Math|Vector|MakeVector _output_get (Variables|Default|GetYOffset) _output_get_2) false false)
      (Transformation|SetActorRotation (Math|Rotator|MakeRotator 0.0 -5.0 (.yaw (Math|Rotator|FindLookatRotation (Transformation|GetActorLocation) (Transformation|GetActorLocation (Variables|Default|GetActorFollow)))))))))

(fn GetNewXValue
  (bind _actorfollow (Variables|Default|GetActorFollow))
  (bind _actorfollow_2 (Variables|Default|GetActorFollow))
  (bind _xdead_zone (Variables|Default|GetXDead_Zone))
  (bind _xdead_zone_2 (Variables|Default|GetXDead_Zone))
  (bind _returnvalue (Transformation|GetActorLocation _actorfollow))
  (bind _returnvalue_2 (Transformation|GetActorLocation _actorfollow_2))
  (bind _returnvalue_3 (- (.x _returnvalue_2) _xdead_zone))
  (bind _returnvalue_4 (+ (.x _returnvalue) _xdead_zone_2))
  (if (> _returnvalue_3 (.x (Transformation|GetActorLocation)))
    (return _returnvalue_3)
    (elif (< _returnvalue_4 (.x (Transformation|GetActorLocation)))
      (return _returnvalue_4)
      (else
        (return (Variables|Default|GetCameraX))))))

(fn GetNewZValue
  (bind _actorfollow (Variables|Default|GetActorFollow))
  (bind _actorfollow_2 (Variables|Default|GetActorFollow))
  (bind _zdead_zone (Variables|Default|GetZDead_Zone))
  (bind _zdead_zone_2 (Variables|Default|GetZDead_Zone))
  (bind _returnvalue (Transformation|GetActorLocation _actorfollow))
  (bind _returnvalue_2 (Transformation|GetActorLocation _actorfollow_2))
  (bind _returnvalue_3 (- (.z _returnvalue_2) _zdead_zone))
  (bind _returnvalue_4 (+ (.z _returnvalue) _zdead_zone_2))
  (if (!= (Variables|Default|GetFixedZValue) 415.0)
    (return (Variables|Default|GetFixedZValue))
    (elif (> _returnvalue_3 (.z (Transformation|GetActorLocation)))
      (return _returnvalue_3)
      (elif (< _returnvalue_4 (.z (Transformation|GetActorLocation)))
        (return _returnvalue_4)
        (else
          (return (Variables|Default|GetCameraZ)))))))