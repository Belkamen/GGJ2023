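; Pickup item actor that the player collects with the F key, provided its weight fits within the main character's carry limit.
; F adds the item's weight to the character and sends a pickup message with itself and its mesh.
; The PickUp event either copies that mesh onto the character's Object component or enlarges that component, depending on carried weight, then destroys the actor.
; Tick switches off physics simulation once the mesh stops moving.
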(event EventTick
  (params (DeltaSeconds :type Float%20%28single-precision%29))
  (if (<= (Math|Vector|VectorLength (Transformation|GetComponentVelocity (Variables|Default|GetStaticMesh))) 0.0)
    (Utilities|FlowControl|DoOnce false
      (:Completed
        (Physics|SetSimulatePhysics (Variables|Default|GetStaticMesh) false)))))

(event EventPickUp
  (params (Actor :type Actor%20Object%20Reference) (StaticMesh :type Static%20Mesh%20Object%20Reference))
  (bind _as_main_character (Variables|Default|GetAs%20Main%20Character))
  (bind _object (Variables|/Game/Blueprints/Pawns/Main_character.Main_character_C|GetObject _as_main_character))
  (if (<= (Variables|/Game/Blueprints/Pawns/Main_character.Main_character_C|GetWeight _as_main_character) 1)
    (Components|StaticMesh|SetStaticMesh _object StaticMesh)
    (else
      (Transformation|SetWorldScale3D _object (+ (Transformation|GetWorldScale _object) 0.2))))
  (Actor|DestroyActor Actor))

(event Input|KeyboardEvents|F
  (params (Key :type Key%20Structure :default "None"))
  (bind _self self)
  (bind _as_main_character (Variables|Default|GetAs%20Main%20Character))
  (bind _as_main_character_2 (Variables|Default|GetAs%20Main%20Character))
  (:Pressed
    (if (not (> (+ (Variables|Default|GetObjectWeight) (Variables|/Game/Blueprints/Pawns/Main_character.Main_character_C|GetWeight _as_main_character_2)) (Variables|/Game/Blueprints/Pawns/Main_character.Main_character_C|GetMaxWeight _as_main_character_2)))
      (Variables|/Game/Blueprints/Pawns/Main_character.Main_character_C|SetWeight _as_main_character (+ (Variables|Default|GetObjectWeight) (Variables|/Game/Blueprints/Pawns/Main_character.Main_character_C|GetWeight _as_main_character)))
      (Class|InteractInterface|PickUp(Message) _self _self (Variables|/Script/Engine.StaticMeshComponent|GetStaticMesh (Variables|Default|GetStaticMesh))))))

(fn ConstructionScript
  (|CallParentFunction))