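; TreeFeed_Trigger is an actor that lets the main character feed carried weight into its health, presumably that of a tree.
; On BeginPlay it registers itself as Owner of the Health widget in its widget component.
; Pressing F while the character's Weight is positive adds double that weight to CurrentHealth, clamped to MaxHealth, then calls RemoveObject on the character.
; The graph contains no overlap check and never assigns the character reference.
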(event EventBeginPlay
  (bind _ashealth (Utilities|Casting|CastToHealth (UserInterface|GetUserWidgetObject (Variables|Default|GetWidget))))
  (Variables|/Game/Blueprints/Widgets/Health.Health_C|SetOwner _ashealth self))

(event Input|KeyboardEvents|F
  (params (Key :type Key%20Structure :default "None"))
  (bind _as_main_character (Variables|Default|GetAs%20Main%20Character))
  (:Pressed
    (if (> (Variables|/Game/Blueprints/Pawns/Main_character.Main_character_C|GetWeight (Variables|Default|GetAs%20Main%20Character)) 0)
      (Variables|Default|SetCurrentHealth (Math|Float|Clamp(Float) (+ (Variables|Default|GetCurrentHealth) (* (Variables|/Game/Blueprints/Pawns/Main_character.Main_character_C|GetWeight _as_main_character) 2)) 0.0 (Variables|Default|GetMaxHealth)))
      (Default|RemoveObject _as_main_character))))

(fn ConstructionScript
  (|CallParentFunction))