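; Player character for a side-scrolling game that moves along one axis, launches upward to jump, and throws a held object toward the mouse cursor.
; Each tick, the cursor ray is intersected with the character's Y plane to rotate the aim arrow and flip the mesh to match.
; Left click, when Weight is above zero, spawns a weighted Projectile at Arrow3 with the object's scale, then clears the held object.
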(event Custom|GetCursorPosition
  (bind _returnvalue (Game|GetPlayerController 0))
  (bind _mesh (Variables|Character|GetMesh))
  (bind _arrow1 (Variables|Default|GetArrow1))
  (bind (_worldlocation _worlddirection) (Game|Player|ConvertMouseLocationToWorldSpace _returnvalue))
  ;[0 0 0] AimRotation
  (bind _returnvalue_2 (CallFunction|AimLocation _worldlocation (+ _worldlocation (* _worlddirection 1e+04))))
  (bind _output_get (Variables|Default|SetYaw (.Yaw (Math|Vector|GetYawPitchfromVector (Math|Vector|Normalize (- _returnvalue_2 (Transformation|GetWorldLocation (Variables|Default|GetArrow1))))))))
  (bind _output_get_2 (Variables|Default|SetPitch (.Pitch (Math|Vector|GetYawPitchfromVector (Math|Vector|Normalize (- _returnvalue_2 (Transformation|GetWorldLocation (Variables|Default|GetArrow1))))))))
  (Transformation|SetRelativeRotation _arrow1 (Math|Rotator|MakeRotator 0.0 _output_get_2 _output_get) false false)
  ;[1 1 1] PlayerRotation
  (if (> (.Yaw (Math|Rotator|BreakRotator (Variables|/Script/Engine.SceneComponent|GetRelativeRotation _arrow1))) 0.0)
    (Transformation|SetRelativeRotation _mesh "0.000000,180.000000,0.000000" false false)
    (else
      (Transformation|SetRelativeRotation _mesh "0.000000,0.000000,0.000000" false false))))

(event Custom|ThrowObject
  (bind _arrow3 (Variables|Default|GetArrow3))
  ;[0.4635 0.4635 0.4635] ThrowObjectSystem
  (if (> (Variables|Default|GetWeight) 0)
    (Game|SpawnActorfromClass "/Game/Blueprints/Actors/Projectile.Projectile_C" (Math|Transform|MakeTransform (Transformation|GetWorldLocation _arrow3) (Transformation|GetWorldRotation _arrow3) (Transformation|GetWorldScale (Variables|Default|GetObject))) "AlwaysSpawn" self (Variables|Default|GetWeight) 0)
    (CallFunction|RemoveObject)))

(event Custom|RemoveObject
  (bind _object (Variables|Default|GetObject))
  ;[0.4635 0.4635 0.4635] ThrowObjectSystem
  (Variables|Default|SetWeight 0)
  (Components|StaticMesh|SetStaticMesh _object 0)
  (Transformation|SetWorldScale3D _object "2.200000,2.200000,2.200000"))

(event EventTick
  (params (DeltaSeconds :type Float%20%28single-precision%29))
  ;[0 0 0] AimRotation
  (CallFunction|GetCursorPosition))

(event Input|ActionEvents|InputActionJump
  (params (Key :type Key%20Structure :default "None"))
  ;[1 1 1] Movements
  (:Pressed
    (Character|LaunchCharacter "0.000000,0.000000,1500.000000" false true)))

(event Input|AxisEvents|InputAxisMoveRight
  (params (AxisValue :type Float%20%28single-precision%29))
  ;[1 1 1] Movements
  (Pawn|Input|AddMovementInput (Math|Vector|GetForwardVector (Math|Rotator|MakeRotator 0.0 0.0 (.Yaw (Math|Rotator|BreakRotator (Pawn|GetControlRotation :!class /Script/Engine.Pawn))))) AxisValue false))

(event Input|MouseEvents|LeftMouseButton
  (params (Key :type Key%20Structure :default "None"))
  ;[0.4635 0.4635 0.4635] ThrowObjectSystem
  (:Pressed
    (CallFunction|ThrowObject)))

(fn ConstructionScript)

(fn AimLocation
  (params (InputLocation :type Vector) (InputPin :type Vector))
  (bind _returnvalue (Transformation|GetActorLocation))
  (bind (_x _y _z) (Math|Vector|BreakVector InputPin))
  (bind (_x_2 _y_2 _z_2) (Math|Vector|BreakVector InputLocation))
  (return (Math|Vector|MakeVector (+ (/ (* (- (.y _returnvalue) _y_2) (- _x _x_2)) (- _y _y_2)) _x_2) (.y _returnvalue) (+ _z_2 (/ (* (- (.y _returnvalue) _y_2) (- _z _z_2)) (- _y _y_2))))))